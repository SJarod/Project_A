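; MainCamera is a camera actor that becomes the player controller's view target and follows the player horizontally.
; On BeginPlay it takes the controller from FollowPlayer.Player, sets itself as view target and snaps its SpringArm to the player's location.
; Each Tick it lerps the actor toward the player's X and Y by FollowSpeed, keeping its own Z.
; The lerp alpha ignores delta time, so smoothing depends on frame rate.
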(event EventBeginPlay
  (bind _asplayer_controller (Utilities|Casting|CastToPlayerController (Pawn|GetController (Variables|/Script/Project_A4.FollowPlayer|Getplayer (Variables|Default|GetFollowPlayer)))))
  (Game|Player|SetViewTargetwithBlend _asplayer_controller self 0.0 "VTBlend_Linear" 0.0 false)
  ;[1 1 1] Snap spring arm to player target
  (Transformation|SetWorldLocation (Variables|Default|GetSpringArm) (Transformation|GetActorLocation (Variables|/Script/Project_A4.FollowPlayer|Getplayer (Variables|Default|GetFollowPlayer))) false false))

(event Collision|EventActorBeginOverlap
  (params (OtherActor :type Actor%20Object%20Reference)))

(event EventTick
  (params (DeltaSeconds :type Float%20%28single-precision%29))
  (bind _followplayer (Variables|Default|GetFollowPlayer))
  (bind _player (Variables|/Script/Project_A4.FollowPlayer|Getplayer _followplayer))
  (bind _returnvalue (Transformation|GetActorLocation _player))
  ;[1 1 1] Follow target
  (Transformation|SetActorLocation (Math|Vector|Lerp(Vector) (Transformation|GetActorLocation) (Math|Vector|MakeVector (.x _returnvalue) (.y _returnvalue) (.z (Transformation|GetActorLocation))) (Variables|Default|GetFollowSpeed)) false false))

(fn ConstructionScript)